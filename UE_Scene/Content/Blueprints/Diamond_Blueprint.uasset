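; Diamond actor that moves itself whenever IOB_Diamond fires its OnParamChanged event.
; Each event adds an offset to the current location, a fixed step in X and the received value in Y and Z, so movement accumulates.
; It then passes double the value to IOB's UpdateParam and prints debug messages.
; An actor-scaling node driven by the same value is left unconnected, and the construction script is empty.
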(event OnParamChanged(IOB_Diamond)
  (params (ParamValue :type Float%20%28single-precision%29))
  (Transformation|SetActorLocation (+ (Math|Vector|MakeVector 1.0 ParamValue ParamValue) (Transformation|GetActorLocation)) false false)
  (Development|PrintString (Utilities|String|ToString(Float) ParamValue))
  (Class|IOBehaviorComponent|UpdateParam (Variables|Default|GetIOB) (* ParamValue 2.0))
  (Development|PrintString "Diam_location changed"))

(fn ConstructionScript)