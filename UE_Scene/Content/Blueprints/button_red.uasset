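; Clickable red button actor that toggles a point light and reports its on/off state.
; BeginPlay enables click events on the player controller.
; Clicking the Cube toggles the PointLight's visibility, flips Var between 0 and 1, and passes that value to IOBRedButton via UpdateParam.
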(event OnClicked(Cube)
  (params (TouchedComponent :type Primitive%20Component%20Object%20Reference) (ButtonPressed :type Key%20Structure :default "None"))
  (bind _iob_red_button (Variables|Default|GetIOB_red_button))
  (Rendering|ToggleVisibility (Variables|Default|GetPointLight) false)
  (if (== (Variables|Default|Getvar) 0)
    (Variables|Default|Setvar 1)
    (Class|IOBehaviorComponent|UpdateParam _iob_red_button 1.0)
    (else
      (Variables|Default|Setvar 0)
      (Class|IOBehaviorComponent|UpdateParam _iob_red_button 0.0))))

(event EventBeginPlay
  (Variables|/Script/Engine.PlayerController|SetbEnableClickEvents (Game|GetPlayerController 0) true))

(fn ConstructionScript)